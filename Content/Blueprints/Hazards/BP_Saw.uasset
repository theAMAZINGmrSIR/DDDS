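; BP_Saw is a saw blade hazard that deals fixed damage to any actor overlapping its box.
; The overlap also plays a sawing sound, spawned at the world origin rather than at the saw.
; BeginPlay caches the blade's relative location and starts MoveTimeline.
; A separate Move_Timeline update would lerp the blade along local X from that start, but it is marked as never run.
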(event `self.ReceiveBeginPlay`
  (set `self.Start Location` (`SceneComponent.RelativeLocation` (`self.SM_SawBlade`)))
  (`TimelineComponent.PlayFromStart` (`self.Move_Timeline`)))

(event `self.Box.OnComponentBeginOverlap`
  (params (OverlappedComponent :type "PrimitiveComponent Object Reference") (OtherActor :type "Actor Object Reference") (OtherComp :type "PrimitiveComponent Object Reference") (OtherBodyIndex :type Integer) (bFromSweep :type Boolean) (SweepResult :type "HitResult Structure (by ref)"))
  (`GameplayStatics.ApplyDamage` OtherActor 25.0)
  (`GameplayStatics.SpawnSoundAtLocation` "/Game/Sounds_Pack/cue/Sawing_Wood_1-1_Cue.Sawing_Wood_1-1_Cue" (0.0 0.0 0.0) (struct) 1.0 1.0 0.0 null null))

(fn `UserConstructionScript`)