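; BP_Saw_Blade is a moving saw hazard that damages any actor overlapping its Box component.
; On BeginPlay, a timeline slides the Sphere component along relative X from the Scene component's relative location, reversing at each end to loop back and forth.
; Box overlap applies fixed damage and spawns a sawing sound at the world origin rather than at the blade.
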(event `move`
  (bind _move_timeline (`self.Move_Timeline`))
  (bind (_start_location_x _start_location_y _start_location_z) (`KismetMathLibrary.BreakVector` (`self.Start Location`)))
  (set `self.Start Location` (`SceneComponent.RelativeLocation` (`self.Scene`)))
  (bind (_direction _newtrack_1) (`Timeline|Move_Timeline`)
    (:`Update`
      (`SceneComponent.K2_SetRelativeLocation` (`self.Sphere`) (`KismetMathLibrary.VLerp` (`self.Start Location`) (`KismetMathLibrary.MakeVector` (+ _start_location_x 250.0) _start_location_y _start_location_z) _newtrack_1) false false))
    (:`Finished`
      (if (`|EnumEquality` _direction "Forward")
        (`TimelineComponent.Reverse` _move_timeline)
        (else
          (`TimelineComponent.Play` _move_timeline))))))

(event `self.ReceiveBeginPlay`
  (`self.move`))

(event `self.Box.OnComponentBeginOverlap`
  (params (OverlappedComponent :type "PrimitiveComponent Object Reference") (OtherActor :type "Actor Object Reference") (OtherComp :type "PrimitiveComponent Object Reference") (OtherBodyIndex :type Integer) (bFromSweep :type Boolean) (SweepResult :type "HitResult Structure (by ref)"))
  (`GameplayStatics.ApplyDamage` OtherActor 25.0)
  (`GameplayStatics.SpawnSoundAtLocation` "/Game/Sounds_Pack/cue/Sawing_Wood_1-1_Cue.Sawing_Wood_1-1_Cue" (0.0 0.0 0.0) (struct) 1.0 1.0 0.0 null null))

(fn `UserConstructionScript`)